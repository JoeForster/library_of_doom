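; AI controller for the Librarian enemy that runs BT_Librarian on possess and feeds its Blackboard from AI Perception.
; Sighting the player clears the grace timer and sets line of sight and target actor.
; Any other sight update starts that timer, which clears line of sight on expiry but still writes the target actor.
; Non-sight senses, treated as hearing, flag player noise, record its location and store the 2D distance to it.
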(event `self.ReceivePossess`
  (params (PossessedPawn :type "Pawn Object Reference"))
  (`self.RunBehaviorTree` "/Game/LibraryOfDoom/AI/BT_Librarian.BT_Librarian"))

(event `self.AIPerception.OnTargetPerceptionUpdated`
  (params (Actor :type "Actor Object Reference") (Stimulus :type "AIStimulus Structure"))
  (bind (_age _expirationage _strength _stimuluslocation _receiverlocation _tag _bsuccessfullysensed) (break `AIStimulus` Stimulus))
  (bind _blackboard (`self.Blackboard`))
  (bind _hasheardplayer (`self.HasHeardPlayer`))
  (bind _blackboard_2 (`self.Blackboard`))
  (bind _returnvalue (and (`self.ActorHasTag` Actor "Player") _bsuccessfullysensed))
  ;[1 1 1] Perceive Player Stimulus
  (bind _returnvalue_2 (`AIPerceptionSystem.GetSenseClassForStimulus` Stimulus))
  (if (== _returnvalue_2 "/Script/AIModule.AISense_Sight")
    (if _returnvalue
      (`KismetSystemLibrary.K2_ClearAndInvalidateTimerHandle` (`self.Enemy Timer`))
      (`BlackboardComponent.SetValueAsBool` _blackboard (`self.HasLineOfSight`) true)
      (`BlackboardComponent.SetValueAsObject` _blackboard (`self.TargetActor`) Actor)
      (else
        (bind _returnvalue_3 (`KismetSystemLibrary.K2_SetTimerDelegate` (delegate `Start Enemy Timer`) (`self.Line of Sight Timer`)))
        (set `self.Enemy Timer` _returnvalue_3)))
    (elif _returnvalue
      (`BlackboardComponent.SetValueAsBool` _blackboard_2 _hasheardplayer true)
      (`BlackboardComponent.SetValueAsVector` _blackboard_2 (`self.TargetLKP`) _stimuluslocation)
      (set `self.DistanceToSound` (`KismetMathLibrary.Vector_Distance2D` _stimuluslocation _receiverlocation))
      (else
        (`BlackboardComponent.SetValueAsBool` _blackboard_2 _hasheardplayer false)))))

(event `Start Enemy Timer`
  (bind _blackboard (`self.Blackboard`))
  (`BlackboardComponent.SetValueAsBool` _blackboard (`self.HasLineOfSight`) false)
  (`BlackboardComponent.SetValueAsObject` _blackboard (`self.TargetActor`) (stale `self.AIPerception.OnTargetPerceptionUpdated` Actor)))

(fn `UserConstructionScript`)